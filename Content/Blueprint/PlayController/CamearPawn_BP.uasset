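; A camera pawn Blueprint that lets the player pan and zoom the view.
; MoveForward and MoveRight axis inputs feed FloatingPawnMovement along world X and Y, independent of camera facing.
; Zoom actions step the SpringArm length by an increment, clamped between minimum and maximum limits.
; The action names run opposite to arm length: CameraZoomOut shortens the arm and CameraZooMIn lengthens it.
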(event Input|ActionEvents|InputActionCameraZooMIn
  (params (Key :type Key%20Structure :default "None"))
  (bind _springarm (Variables|Default|GetSpringArm))
  ;[1 1 1] MouseZoom
  (:Pressed
    (if (< (+ (Variables|/Script/Engine.SpringArmComponent|GetTargetArmLength _springarm) (Variables|Camera|GetZoomIncrement)) (Variables|Camera|GetMaxZoom))
      (Variables|/Script/Engine.SpringArmComponent|SetTargetArmLength _springarm (+ (Variables|/Script/Engine.SpringArmComponent|GetTargetArmLength _springarm) (Variables|Camera|GetZoomIncrement)))
      (else
        (Variables|/Script/Engine.SpringArmComponent|SetTargetArmLength _springarm (Variables|Camera|GetMaxZoom))))))

(event Input|ActionEvents|InputActionCameraZoomOut
  (params (Key :type Key%20Structure :default "None"))
  (bind _springarm (Variables|Default|GetSpringArm))
  ;[1 1 1] MouseZoom
  (:Pressed
    (if (< (Variables|Camera|GetMinZoom) (- (Variables|/Script/Engine.SpringArmComponent|GetTargetArmLength _springarm) (Variables|Camera|GetZoomIncrement)))
      (Variables|/Script/Engine.SpringArmComponent|SetTargetArmLength _springarm (- (Variables|/Script/Engine.SpringArmComponent|GetTargetArmLength _springarm) (Variables|Camera|GetZoomIncrement)))
      (else
        (Variables|/Script/Engine.SpringArmComponent|SetTargetArmLength _springarm (Variables|Camera|GetMinZoom))))))

(event Input|AxisEvents|InputAxisMoveForward
  (params (AxisValue :type Float%20%28single-precision%29))
  ;[1 1 1] Move
  (Class|PawnMovementComponent|AddInputVector (Variables|Default|GetFloatingPawnMovement) (Math|Vector|MakeVector AxisValue 0.0 0.0) false))

(event Input|AxisEvents|InputAxisMoveRight
  (params (AxisValue :type Float%20%28single-precision%29))
  ;[1 1 1] Move
  (Class|PawnMovementComponent|AddInputVector (Variables|Default|GetFloatingPawnMovement) (Math|Vector|MakeVector 0.0 AxisValue 0.0) false))

(fn ConstructionScript)