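; Infantry character Blueprint that can be selected and deselected, with a decal showing its selection state.
; Each Select event call flips the Selected flag, prints a debug message and sets the SelectionDecal visibility to match.
; IsSelect returns the current flag, and the construction script is empty.
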(event EventSelect
  (if (Variables|Default|GetbSelected)
    (Variables|Default|SetbSelected false)
    (Development|PrintString "Hello")
    (else
      (Variables|Default|SetbSelected true)
      (Development|PrintString "Select" true true "(R=1.000000,G=0.011239,B=0.809112,A=1.000000)")))
  (Rendering|SetVisibility (Variables|Default|GetSelectionDecal) (Variables|Default|GetbSelected) false))

(fn ConstructionScript)

(fn IsSelect
  (return (Variables|Default|GetbSelected)))